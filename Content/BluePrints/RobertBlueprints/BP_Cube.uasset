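; BP_Cube is a physics cube that can dissolve by sinking below where it was and then respawn.
; Dissolve, guarded against re-entry until the sink ends, disables overlaps and physics, waits, then runs a timeline easing the mesh downward from its current location.
; It then hides the mesh and, after a delay, restores it at the Scene component's location and rotation with physics and overlaps on.
; Shake wakes the rigid body.
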(event `/Game/BluePrints/RobertBlueprints/BPI_Interactables.Dissolve`
  (bind _mesh (`self.Mesh`))
  (bind (_returnvalue_location _returnvalue_rotation) (`KismetMathLibrary.BreakTransform` (`SceneComponent.K2_GetComponentToWorld` (`self.Scene`))))
  ;[1 1 1] "Dissolve" the object and respawn it after x-time
  (if (not (`self.Dissolving`))
    (set `self.OverlapLocation` (`SceneComponent.K2_GetComponentLocation` (`self.Mesh`)))
    (set `self.Dissolving` true)
    (set `PrimitiveComponent.bGenerateOverlapEvents` false (`self.Mesh`))
    (`PrimitiveComponent.SetSimulatePhysics` (`self.Mesh`) false)
    (`KismetSystemLibrary.Delay` (`self.DissolveDelay`))
    (bind (_direction _dissolve) (`Timeline|Sink Through the ground` :!via `PlayFromStart`)
      (:`Update`
        (`SceneComponent.K2_SetWorldLocation` (`self.Mesh`) (`|EaseFunction` "EaseInOut" _dissolve (`SceneComponent.K2_GetComponentLocation` (`self.Mesh`)) (+ (`self.OverlapLocation`) (0.0 0.0 -200.0))) false true))
      (:`Finished`
        (set `self.Dissolving` false)
        (`SceneComponent.SetHiddenInGame` (`self.Mesh`) true false)
        (`KismetSystemLibrary.Delay` (`self.RespawnDelay`))
        (`SceneComponent.K2_SetWorldTransform` (`self.Mesh`) (`KismetMathLibrary.MakeTransform` _returnvalue_location _returnvalue_rotation (`SceneComponent.K2_GetComponentScale` (`self.Mesh`))) false true)
        (`PrimitiveComponent.SetSimulatePhysics` _mesh true)
        (`SceneComponent.SetHiddenInGame` _mesh false false)
        (set `PrimitiveComponent.bGenerateOverlapEvents` true (`self.Mesh`))))))

(event `/Game/BluePrints/RobertBlueprints/BPI_Interactables.Shake`
  ;[1 1 1] Awake the Rigid body
  (`PrimitiveComponent.WakeRigidBody` (`self.Mesh`) "None"))

(fn `UserConstructionScript`)