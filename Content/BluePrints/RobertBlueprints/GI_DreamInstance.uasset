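; GI_DreamInstance is a game instance that holds the player's audio and mouse sensitivity settings.
; Update events store master volume, SFX volume and mouse sensitivity in its variables.
; Two Send functions return those stored values to callers.
; It only stores values and does not apply them to audio or input itself.
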(event `/Game/BluePrints/RobertBlueprints/BPI_GameInstance.Update Volume Settings`
  (params (`Master Volume` :type "Float (double-precision)") (`SFX Volume` :type "Float (double-precision)"))
  (set `self.Master Volume` `Master Volume`)
  (set `self.SFX Volume` `SFX Volume`))

(event `/Game/BluePrints/RobertBlueprints/BPI_GameInstance.Update Mouse Sensitivity`
  (params (MouseSensitivity :type "Float (double-precision)"))
  (set `self.Mouse Sensitivity` MouseSensitivity))

(fn `Send Mouse Sensitivity`
  (returns (`Mouse Sensitivity` :type "Float (double-precision)"))
  (return (`self.Mouse Sensitivity`)))

(fn `Send Volume Settings`
  (returns (`Master Volume` :type "Float (double-precision)") (`SFX Volume` :type "Float (double-precision)"))
  (return (`self.Master Volume`) (`self.SFX Volume`)))