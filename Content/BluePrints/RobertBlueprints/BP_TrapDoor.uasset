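; Two-door trap door that swings open and closed through its T7InteractableResponse activate and deactivate events.
; Stores both doors' starting rotations on BeginPlay, then the OpenCloseDoors timeline eases each toward -90 pitch, keeping its roll and yaw.
; Deactivation reverses the same timeline to close them.
; Any actor leaving the Box volume is sent ShakeMessage, independently of the door state.
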(event `self.ReceiveBeginPlay`
  (set `self.StartRotation1` (`SceneComponent.RelativeRotation` (`self.Door1`)))
  (set `self.StartRotation2` (`SceneComponent.RelativeRotation` (`self.Door2`))))

(event `self.T7InteractableResponse.OnActivate`
  (bind (_startrotation1_roll _startrotation1_pitch _startrotation1_yaw) (`KismetMathLibrary.BreakRotator` (`self.StartRotation1`)))
  (bind (_startrotation2_roll _startrotation2_pitch _startrotation2_yaw) (`KismetMathLibrary.BreakRotator` (`self.StartRotation2`)))
  (bind (_direction _open) (`Timeline|Open & Close Doors` :!label _label)
    (:`Update`
      (`SceneComponent.K2_SetRelativeRotation` (`self.Door1`) (`|EaseFunction` "EaseInOut" _open (`self.StartRotation1`) (`KismetMathLibrary.MakeRotator` _startrotation1_roll -90.0 _startrotation1_yaw)) false true)
      (`SceneComponent.K2_SetRelativeRotation` (`self.Door2`) (`|EaseFunction` "EaseInOut" _open (`self.StartRotation2`) (`KismetMathLibrary.MakeRotator` _startrotation2_roll -90.0 _startrotation2_yaw)) false false))))

(event `self.T7InteractableResponse.OnDeactivate`
  (goto _label :!via `Reverse`))

(event `self.Box.OnComponentEndOverlap`
  (params (OverlappedComponent :type "PrimitiveComponent Object Reference") (OtherActor :type "Actor Object Reference") (OtherComp :type "PrimitiveComponent Object Reference") (OtherBodyIndex :type Integer))
  (message `/Game/BluePrints/RobertBlueprints/BPI_Interactables.Shake` OtherActor))

(fn `UserConstructionScript`)