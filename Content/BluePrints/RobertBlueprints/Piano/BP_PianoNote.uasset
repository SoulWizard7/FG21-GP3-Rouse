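; BP_PianoNote is a single piano key that the player can press or that plays itself during songs.
; On box overlap it sends DissolveMessage to the other actor, tilts via a timeline and reports its note to MyPiano as player input.
; PlaySong matches the number against three song slots, waits that slot's delay, then animates likewise and reports a song note.
; A shared Reverse flag makes each press report once before springing back.
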(event `self.Box.OnComponentBeginOverlap`
  (params (OverlappedComponent :type "PrimitiveComponent Object Reference") (OtherActor :type "Actor Object Reference") (OtherComp :type "PrimitiveComponent Object Reference") (OtherBodyIndex :type Integer) (bFromSweep :type Boolean) (SweepResult :type "HitResult Structure (by ref)"))
  (bind (_relativerotation_roll _relativerotation_pitch _relativerotation_yaw) (`KismetMathLibrary.BreakRotator` (`SceneComponent.RelativeRotation` (`self.DefaultSceneRoot`))))
  (bind (_relativerotation_roll_2 _relativerotation_pitch_2 _relativerotation_yaw_2) (`KismetMathLibrary.BreakRotator` (`SceneComponent.RelativeRotation` (`self.DefaultSceneRoot`))))
  (message `/Game/BluePrints/RobertBlueprints/BPI_Interactables.Dissolve` OtherActor)
  ;[1 1 1] Player have pressed a key
  (`TimelineComponent.SetPlayRate` (`self.Player Played Note`) 10.0)
  (bind (_direction _push_down) (`Timeline|Player Played Note` :!via `PlayFromStart` :!label _label)
    (:`Update`
      (`SceneComponent.K2_SetRelativeRotation` (`self.DefaultSceneRoot`) (`|EaseFunction` "Linear" _push_down (`KismetMathLibrary.MakeRotator` _relativerotation_roll_2 0.0 _relativerotation_yaw_2) (`KismetMathLibrary.MakeRotator` _relativerotation_roll -5.0 _relativerotation_yaw)) false false))
    (:`Finished`
      (if (`self.Reverse?`)
        (set `self.Reverse?` false)
        (else
          (set `self.Reverse?` true)
          (message `/Game/BluePrints/RobertBlueprints/Piano/BPI_Piano.PlayerNoteOrder` (`self.MyPiano`) (`self.Note`))
          (`KismetSystemLibrary.Delay` 0.01)
          (goto _label :!via `ReverseFromEnd`))))))

(event `/Game/BluePrints/RobertBlueprints/Piano/BPI_Piano.PlaySong`
  (params (SongNumber :type Integer))
  (bind (_relativerotation_roll _relativerotation_pitch _relativerotation_yaw) (`KismetMathLibrary.BreakRotator` (`SceneComponent.RelativeRotation` (`self.DefaultSceneRoot`))))
  (bind (_relativerotation_roll_2 _relativerotation_pitch_2 _relativerotation_yaw_2) (`KismetMathLibrary.BreakRotator` (`SceneComponent.RelativeRotation` (`self.DefaultSceneRoot`))))
  ;[1 1 1] Check if this note is suppose to be played. (And if yes, when)
  (if (== SongNumber (`self.Song1`))
    (`KismetSystemLibrary.Delay` (`self.Song1Delay`))
    ;[1 1 1] Key is pressed (Song is being played)
    (`TimelineComponent.SetPlayRate` (`self.Press down note`) 10.0 :!label _label_2)
    (bind (_direction _press_down_note) (`Timeline|Press down note` :!via `PlayFromStart` :!label _label_3)
      (:`Update`
        (`SceneComponent.K2_SetRelativeRotation` (`self.DefaultSceneRoot`) (`|EaseFunction` "Linear" _press_down_note (`KismetMathLibrary.MakeRotator` _relativerotation_roll 0.0 _relativerotation_yaw) (`KismetMathLibrary.MakeRotator` _relativerotation_roll_2 -5.0 _relativerotation_yaw_2)) false false))
      (:`Finished`
        (if (`self.Reverse?`)
          (set `self.Reverse?` false)
          (else
            (set `self.Reverse?` true)
            (message `/Game/BluePrints/RobertBlueprints/Piano/BPI_Piano.SongNoteOrder` (`self.MyPiano`) (`self.Note`))
            (`KismetSystemLibrary.Delay` 0.01)
            (goto _label_3 :!via `ReverseFromEnd`)))))
    (elif (== SongNumber (`self.Song2`))
      (`KismetSystemLibrary.Delay` (`self.Song2Delay`))
      (goto _label_2)
      (elif (== SongNumber (`self.Song3`))
        (`KismetSystemLibrary.Delay` (`self.Song3Delay`))
        (goto _label_2)))))

(fn `PlayNote`
  (return))

(fn `UserConstructionScript`)