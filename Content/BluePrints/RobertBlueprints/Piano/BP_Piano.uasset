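; BP_Piano is a piano puzzle where the player repeats numbered songs by playing notes in the correct order.
; PlaySong messages every linked key with the current song number, guarded by a five-second busy flag.
; SongNoteOrder records unique notes as the expected sequence, and PlayerNoteOrder collects input until lengths match.
; A matching sequence advances the displayed song number or completes the puzzle, while a mismatch clears the player's input.
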(event `self.ReceiveBeginPlay`
  ;[1 1 1] Show text of what song that is to be played
  (`TextRenderComponent.K2_SetText` (`self.TextRender`) (`KismetTextLibrary.Conv_IntToText` (`self.SongNumber`))))

(event `/Game/BluePrints/RobertBlueprints/Piano/BPI_Piano.PlaySong`
  (params (SongNumber :type Integer))
  ;[1 1 1] Play song if puzzle not yet complete (Call all notes associated with this piano)
  (if (not (`self.IsPlaying`))
    (set `self.IsPlaying` true)
    (if (not (`self.PuzzleComplete`))
      (for _array_element (`self.PianoKeys`)
        (message `/Game/BluePrints/RobertBlueprints/Piano/BPI_Piano.PlaySong` _array_element (`self.SongNumber`)))
      (`KismetSystemLibrary.Delay` 5.0)
      (set `self.IsPlaying` false))))

(event `/Game/BluePrints/RobertBlueprints/Piano/BPI_Piano.SongNoteOrder`
  (params (Note :type String))
  ;[1 1 1] Adding notes & note order of song to Array
  (`KismetArrayLibrary.Array_AddUnique` (`self.SongNotesOrder`) Note))

(event `/Game/BluePrints/RobertBlueprints/Piano/BPI_Piano.PlayerNoteOrder`
  (params (Note :type String))
  (bind _songnotesorder (`self.SongNotesOrder`))
  (bind _returnvalue (== (`KismetArrayLibrary.Array_Length` (`self.PlayerNotesOrder`)) (`KismetArrayLibrary.Array_Length` (`self.SongNotesOrder`))))
  ;[1 1 1] Creating the Array of player played notes
  (if (`KismetArrayLibrary.Array_IsValidIndex` _songnotesorder (- (`KismetArrayLibrary.Array_Length` _songnotesorder) 1))
    (if _returnvalue
      (`self.Check If Played Notes Are Correct`)
      (else
        (`KismetArrayLibrary.Array_Add` (`self.PlayerNotesOrder`) Note)
        (if _returnvalue
          (`self.Check If Played Notes Are Correct`))))))

(event `Check If Played Notes Are Correct`
  ;[1 1 1] Update Song to play (if last song have not been completed)
  (if (`KismetArrayLibrary.Array_Identical` (`self.PlayerNotesOrder`) (`self.SongNotesOrder`))
    (`KismetArrayLibrary.Array_Clear` (`self.PlayerNotesOrder`))
    (`KismetArrayLibrary.Array_Clear` (`self.SongNotesOrder`))
    (`KismetSystemLibrary.PrintString` "CORRECT!")
    (if (< (`self.SongNumber`) (`self.LastSongNumber`))
      (`/Engine/EditorBlueprintResources/StandardMacros.IncrementInt` (`self.SongNumber`)
        (:`  `
          (`TextRenderComponent.K2_SetText` (`self.TextRender`) (`KismetTextLibrary.Conv_IntToText` (`self.SongNumber`)))))
      (else
        (`KismetSystemLibrary.PrintString` "PIANO COMPLETE!")
        (set `self.PuzzleComplete` true)))
    (else
      (`KismetArrayLibrary.Array_Clear` (`self.PlayerNotesOrder`))
      (`KismetSystemLibrary.PrintString` "FAILED"))))

(fn `PlayNote`
  (return))

(fn `UserConstructionScript`)