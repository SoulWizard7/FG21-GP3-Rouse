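; BP_PowerSensitiv is an object that reacts to the levitation power by moving its mesh to a target position and back.
; BeginPlay caches the mesh's relative location as the start point.
; On levitation start it deactivates the box and plays a timeline that linearly lerps the mesh to a scene component's location.
; After a PowerLength delay the timeline reverses, with IsAnimating and HaveReset flags blocking retriggers until it returns.
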(event `self.ReceiveBeginPlay`
  ;[1 1 1] Begin play (Saving the relative location fo Mesh)
  (set `self.MeshRelativeLocation` (`SceneComponent.RelativeLocation` (`self.Mesh`))))

(event `self.T7LevitateResponse.OnStartLevitate`
  ;[1 1 1] Affected by levitation power
  (`ActorComponent.Deactivate` (`self.Box`))
  (if (not (`self.IsAnimating`))
    (set `self.IsAnimating` true)
    (bind (_direction _test) (`Timeline|Move` :!label _label)
      (:`Update`
        (`SceneComponent.K2_SetRelativeLocation` (`self.Mesh`) (`|EaseFunction` "Linear" _test (`self.MeshRelativeLocation`) (`SceneComponent.RelativeLocation` (`self.Scene`))) false false))
      (:`Finished`
        (if (`self.HaveReset?`)
          (set `self.HaveReset?` false)
          (set `self.IsAnimating` false)
          (else
            (`KismetSystemLibrary.Delay` (`self.PowerLength`))
            (set `self.HaveReset?` true)
            (goto _label :!via `Reverse`)))))))

(fn `UserConstructionScript`)