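; BP_RetractExplanation is a trigger actor that shows a one-time explanation screen for the retract mechanic.
; When the player character first overlaps its Box, it creates and displays the Retcract widget and sets HasSeenRetract so it does not repeat.
; It then switches to UI-only input with a visible cursor, sets CanSeePush and pauses the game.
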(event `self.Box.OnComponentBeginOverlap`
  (params (OverlappedComponent :type "PrimitiveComponent Object Reference") (OtherActor :type "Actor Object Reference") (OtherComp :type "PrimitiveComponent Object Reference") (OtherBodyIndex :type Integer) (bFromSweep :type Boolean) (SweepResult :type "HitResult Structure (by ref)"))
  (bind _returnvalue (`GameplayStatics.GetPlayerController` 0))
  (if (== OtherActor (`GameplayStatics.GetPlayerCharacter` 0))
    (if (not (`self.HasSeenRetract`))
      (bind _returnvalue_2 (`|CreateWidget` "/Game/_Game/UI/Widgets/Retcract.Retcract_C"))
      (set `self.Widget` _returnvalue_2)
      (`UserWidget.AddToViewport` _returnvalue_2 0)
      (set `self.HasSeenRetract` true)
      (`WidgetBlueprintLibrary.SetInputMode_UIOnlyEx` _returnvalue null)
      (set `PlayerController.bShowMouseCursor` true _returnvalue)
      (set `self.CanSeePush` true)
      (`GameplayStatics.SetGamePaused` true))))

(fn `UserConstructionScript`)