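; Prototype moving platform that rises and lowers in response to T7 interactable activation.
; Activation plays a timeline that linearly moves MovingPlatform 500 units up along relative Z, without sweep, and deactivation reverses it.
; Each timeline update also unhides the Cylinder, which is never hidden again here.
; A second timeline for the downward move is left unconnected and never runs.
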(event `self.T7InteractableResponse.OnActivate`
  (bind (_direction _move) (`Timeline|Timeline_0` :!label _label)
    (:`Update`
      (`SceneComponent.K2_SetRelativeLocation` (`self.MovingPlatform`) (`|EaseFunction` "Linear" _move (0.0 0.0 0.0) (0.0 0.0 500.0)) false false)
      (`SceneComponent.SetHiddenInGame` (`self.Cylinder`) false false))))

(event `self.T7InteractableResponse.OnDeactivate`
  (goto _label :!via `Reverse`))

(fn `UserConstructionScript`)