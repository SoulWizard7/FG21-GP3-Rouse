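; BP_Wires is a spline-shaped wire actor with a swaying fluid material that switches color to show active or inactive state.
; The construction script builds a spline mesh per segment, giving each a dynamic material set from exposed color, brightness and sway variables.
; ActivateColor and DeactivateColor loop over the stored meshes, apply a material from the last saved MatInstance and set its fluid color green or red.
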(event `/Game/BluePrints/RobertBlueprints/BPI_Interactables.ActivateColor`
  (for _array_element (`self.Mesh Array`)
    (bind _returnvalue (`PrimitiveComponent.CreateDynamicMaterialInstance` _array_element 0 (`self.Mat Instance`) "None"))
    (`MaterialInstanceDynamic.SetVectorParameterValue` _returnvalue "Fluid Color" (struct :`R` 0.231934 :`G` 0.890625 :`B` 0.477037 :`A` 1.0))))

(event `/Game/BluePrints/RobertBlueprints/BPI_Interactables.DeactivateColor`
  (for _array_element (`self.Mesh Array`)
    (bind _returnvalue (`PrimitiveComponent.CreateDynamicMaterialInstance` _array_element 0 (`self.Mat Instance`) "None"))
    (`MaterialInstanceDynamic.SetVectorParameterValue` _returnvalue "Fluid Color" (struct :`R` 1.0 :`B` 0.057805 :`A` 1.0))))

(fn `UserConstructionScript`
  (bind _mat_instance (`self.Mat Instance`))
  (bind _spline (`self.Spline`))
  (for _index (range (+ (- (`SplineComponent.GetNumberOfSplinePoints` (`self.Spline`)) 2) 1))
    (bind _returnvalue (`AddComponent|NODE_AddSplineMeshComponent-0`))
    (bind _output_get (set `self.SplinePeice` _returnvalue))
    (`KismetArrayLibrary.Array_Add` (`self.Mesh Array`) _output_get)
    (`SplineMeshComponent.SetForwardAxis` _returnvalue "Z" true)
    (bind (_location _tangent) (`SplineComponent.GetLocationAndTangentAtSplinePoint` _spline _index "Local"))
    (bind (_location_2 _tangent_2) (`SplineComponent.GetLocationAndTangentAtSplinePoint` _spline (+ _index 1) "Local"))
    (`SplineMeshComponent.SetStartAndEnd` _returnvalue _location _tangent _location_2 _tangent_2 true)
    (bind _returnvalue_2 (`PrimitiveComponent.CreateDynamicMaterialInstance` _returnvalue 0 "/Game/_Game/Art/Materials/M_Spline_Inst.M_Spline_Inst" "None"))
    (set `self.Mat Instance` _returnvalue_2)
    (`|ExecutionSequence`
      (:`then_0`
        (`MaterialInstanceDynamic.SetVectorParameterValue` _mat_instance "Fluid Color" (`self.Fluid Color`)))
      (:`then_1`
        (`MaterialInstanceDynamic.SetScalarParameterValue` _mat_instance "Brightness" (`self.Brightness`)))
      (:`then_2`
        (`MaterialInstanceDynamic.SetScalarParameterValue` _mat_instance "WindIntensity" (`self.Sway Intensity`)))
      (:`then_3`
        (`MaterialInstanceDynamic.SetScalarParameterValue` _mat_instance "WindSpeed" (`self.Sway Speed`))))))