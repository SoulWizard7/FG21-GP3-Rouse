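; BP_GunPickUp is a gun pickup that switches the player character to the gun when touched.
; Overlapping its sphere calls SwitchToGun on BP_T7Character, disables that character's aiming and starts the pickup moving.
; Each tick it then interpolates toward the character's capsule while scaling toward half size, and destroys itself once it is close.
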(event `self.ReceiveTick`
  (params (DeltaSeconds :type "Float (single-precision)"))
  (bind _defaultsceneroot (`self.DefaultSceneRoot`))
  (if (`self.MoveToPlayer`)
    (`SceneComponent.K2_SetWorldLocation` _defaultsceneroot (`KismetMathLibrary.VInterpTo` (`SceneComponent.K2_GetComponentLocation` (`self.DefaultSceneRoot`)) (`SceneComponent.K2_GetComponentLocation` (`Character.CapsuleComponent` (`self.CharacterRef`))) DeltaSeconds 2.0) false false)
    (`SceneComponent.SetRelativeScale3D` _defaultsceneroot (`KismetMathLibrary.VInterpTo` (`SceneComponent.RelativeScale3D` (`self.DefaultSceneRoot`)) (0.5 0.5 0.5) DeltaSeconds 5.0))
    (if (<= (`KismetMathLibrary.Vector_Distance` (`SceneComponent.K2_GetComponentLocation` (`self.DefaultSceneRoot`)) (`SceneComponent.K2_GetComponentLocation` (`Character.CapsuleComponent` (`self.CharacterRef`)))) 50.0)
      (`self.K2_DestroyActor`))))

(event `self.SphereCollision.OnComponentBeginOverlap`
  (params (OverlappedComponent :type "PrimitiveComponent Object Reference") (OtherActor :type "Actor Object Reference") (OtherComp :type "PrimitiveComponent Object Reference") (OtherBodyIndex :type Integer) (bFromSweep :type Boolean) (SweepResult :type "HitResult Structure (by ref)"))
  (bind _asbp_t7character (cast `/Game/_Game/Player/ThirdPersonTest/BP_T7Character` OtherActor))
  (`/Game/_Game/Player/ThirdPersonTest/BP_T7Character.SwitchToGun` _asbp_t7character)
  (bind _output_get (set `self.CharacterRef` _asbp_t7character))
  (set `/Game/_Game/Player/ThirdPersonTest/BP_T7Character.CanAim` false _output_get)
  (set `self.MoveToPlayer` true))

(fn `UserConstructionScript`)