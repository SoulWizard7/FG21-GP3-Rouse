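; A breakable floor plank placeholder that collapses when a triggering actor steps on it.
; When an actor with a T7InteractableTrigger component overlaps the trigger, the geometry collection starts simulating physics, a break sound plays and the intact cube is destroyed.
; After a one-second delay the debris is hidden and loses collision.
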(event `self.Trigger.OnComponentBeginOverlap`
  (params (OverlappedComponent :type "PrimitiveComponent Object Reference") (OtherActor :type "Actor Object Reference") (OtherComp :type "PrimitiveComponent Object Reference") (OtherBodyIndex :type Integer) (bFromSweep :type Boolean) (SweepResult :type "HitResult Structure (by ref)"))
  (bind _cube_geometrycollection (`self.Cube_GeometryCollection`))
  (`/Engine/EditorBlueprintResources/StandardMacros.IsValid` (`self.GetComponentByClass` OtherActor "/Script/GP3.T7InteractableTrigger")
    (:`Is Valid`
      (`PrimitiveComponent.SetSimulatePhysics` (`self.Cube_GeometryCollection`) true)
      (`GameplayStatics.PlaySoundAtLocation` "/Game/_Game/Sounds/SFX/SFX/FloorBreak.FloorBreak" (`SceneComponent.K2_GetComponentLocation` (`self.Trigger`)) (struct) 1.0 1.0 0.0 null null null null)
      (`ActorComponent.K2_DestroyComponent` (`self.Cube`))
      (`KismetSystemLibrary.Delay` 1.0)
      (`SceneComponent.SetHiddenInGame` _cube_geometrycollection true true)
      (`PrimitiveComponent.SetCollisionEnabled` _cube_geometrycollection "NoCollision"))))

(fn `UserConstructionScript`)