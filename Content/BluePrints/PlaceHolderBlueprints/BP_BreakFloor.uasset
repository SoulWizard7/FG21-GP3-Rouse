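; BP_BreakFloor is a placeholder breakable floor that drops the player into the void.
; When an actor with a T7InteractableTrigger component overlaps its Trigger, the geometry collection starts simulating physics and a break sound plays.
; If the solid Cube still exists, it is destroyed, a second sound plays, and player 0's BP_T7Character calls FallToVoid, regardless of which actor triggered it.
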(event `self.Trigger.OnComponentBeginOverlap`
  (params (OverlappedComponent :type "PrimitiveComponent Object Reference") (OtherActor :type "Actor Object Reference") (OtherComp :type "PrimitiveComponent Object Reference") (OtherBodyIndex :type Integer) (bFromSweep :type Boolean) (SweepResult :type "HitResult Structure (by ref)"))
  (`/Engine/EditorBlueprintResources/StandardMacros.IsValid` (`self.GetComponentByClass` OtherActor "/Script/GP3.T7InteractableTrigger")
    (:`Is Valid`
      (`PrimitiveComponent.SetSimulatePhysics` (`self.Cube_GeometryCollection`) true)
      (`GameplayStatics.PlaySoundAtLocation` "/Game/_Game/Sounds/SFX/SFX/FloorBreak.FloorBreak" (`SceneComponent.K2_GetComponentLocation` (`self.Trigger`)) (struct) 1.0 1.0 0.0 null null null null)
      (bind _cube (`self.Cube`)
        (:`then`
          (`ActorComponent.K2_DestroyComponent` _cube)
          (`GameplayStatics.PlaySoundAtLocation` "/Game/_Game/Sounds/Other/Ambience/GameOver_maybe.GameOver_maybe" (0.0 0.0 0.0) (struct) 0.6 1.0 0.0 null null null null)
          (bind _asbp_t7character (cast `/Game/_Game/Player/ThirdPersonTest/BP_T7Character` (`GameplayStatics.GetPlayerPawn` 0)))
          (`/Game/_Game/Player/ThirdPersonTest/BP_T7Character.FallToVoid` _asbp_t7character))
        (:`else`)))))

(fn `UserConstructionScript`)