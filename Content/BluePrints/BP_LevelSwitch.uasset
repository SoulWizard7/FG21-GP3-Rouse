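; Level transition trigger actor that sends the player on to the next map in a hard-coded sequence of test levels.
; When the player character overlaps its Box component, it stores the current level name and checks it through a chain of string comparisons.
; A match opens the paired level by name, while any other level name does nothing.
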(event `self.Box.OnComponentBeginOverlap`
  (params (OverlappedComponent :type "PrimitiveComponent Object Reference") (OtherActor :type "Actor Object Reference") (OtherComp :type "PrimitiveComponent Object Reference") (OtherBodyIndex :type Integer) (bFromSweep :type Boolean) (SweepResult :type "HitResult Structure (by ref)"))
  (bind _currentlevel (`self.CurrentLevel`))
  (if (== OtherActor (`GameplayStatics.GetPlayerCharacter` 0))
    (bind _returnvalue (`GameplayStatics.GetCurrentLevelName` true))
    (set `self.CurrentLevel` _returnvalue)
    (if (`KismetStringLibrary.EqualEqual_StrStr` _currentlevel "Ludwig_Test_Level3")
      (`GameplayStatics.OpenLevel` "TestMap_Marika_LightingTest5")
      (elif (`KismetStringLibrary.EqualEqual_StrStr` _currentlevel "TestMap_Set2")
        (`GameplayStatics.OpenLevel` "Level_3-Sticky2")
        (elif (`KismetStringLibrary.EqualEqual_StrStr` _currentlevel "TestMap_Marika_LightingTest5")
          (`GameplayStatics.OpenLevel` "TestMap_Set2"))))))

(fn `UserConstructionScript`)