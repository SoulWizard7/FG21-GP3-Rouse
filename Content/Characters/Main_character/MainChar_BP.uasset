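; Main player character Blueprint that handles crouch, sprint, aim-down-sights and projectile input.
; Movement inputs set walk speed directly, with crouch also resizing the capsule, ADS narrowing camera FOV, and sprint press ignored while aiming.
; Projectile keys set mutually exclusive Freeze, Sticky and Levitate flags, which are not read in this graph.
; Primary action spawns a scaled-down BP_BulletTest at the capsule, its Z axis aligned to capsule forward.
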(event `InputAction|Crouch`
  (params (Key :type "Key Structure"))
  ;[1 1 1] Crouching
  (:`Pressed`
    (set `CharacterMovementComponent.MaxWalkSpeed` 300.0 (`self.CharacterMovement`))
    (`KismetSystemLibrary.PrintString` "Crouching")
    (`self.Crouch`)
    (`CapsuleComponent.SetCapsuleHalfHeight` (`self.CapsuleComponent`) 45.0 true))
  (:`Released`
    (set `CharacterMovementComponent.MaxWalkSpeed` 500.0 (`self.CharacterMovement`))
    (`KismetSystemLibrary.PrintString` "Not crouching")
    (`self.UnCrouch`)
    (`CapsuleComponent.SetCapsuleHalfHeight` (`self.CapsuleComponent`) 90.0 true)))

(event `InputAction|Projectile1`
  (params (Key :type "Key Structure"))
  ;[1 1 1] Projectile button presses
  (:`Pressed`
    (set `self.bFreeze` true)
    (set `self.bSticky` false)
    (set `self.bLevitate` false)
    (`KismetSystemLibrary.PrintString` "Freezy projectile")))

(event `InputAction|Projectile2`
  (params (Key :type "Key Structure"))
  ;[1 1 1] Projectile button presses
  (:`Pressed`
    (set `self.bFreeze` false)
    (set `self.bLevitate` false)
    (set `self.bSticky` true)
    (`KismetSystemLibrary.PrintString` "Sticky projectile")))

(event `InputAction|Projectile3`
  (params (Key :type "Key Structure"))
  ;[1 1 1] Projectile button presses
  (:`Pressed`
    (set `self.bFreeze` false)
    (set `self.bSticky` false)
    (set `self.bLevitate` true)
    (`KismetSystemLibrary.PrintString` "Levitate projectile")))

(event `InputAction|PrimaryAction`
  (params (Key :type "Key Structure"))
  (bind _capsulecomponent (`self.CapsuleComponent`))
  ;[1 1 1] Shooting
  (:`Pressed`
    (`|SpawnActorFromClass` "/Game/_Game/Projectiles/BP_BulletTest.BP_BulletTest_C" (`KismetMathLibrary.MakeTransform` (`SceneComponent.K2_GetComponentLocation` _capsulecomponent) (`KismetMathLibrary.MakeRotFromZ` (`SceneComponent.GetForwardVector` _capsulecomponent)) (0.2 0.2 0.2)) "Undefined" "OverrideRootScale" null null)))

(event `InputAction|Sprint`
  (params (Key :type "Key Structure"))
  (bind _charactermovement (`self.CharacterMovement`))
  ;[1 1 1] Sprinting
  (:`Pressed`
    (if (not (`self.IsADS`))
      (set `CharacterMovementComponent.MaxWalkSpeed` 450.0 _charactermovement)))
  (:`Released`
    (set `CharacterMovementComponent.MaxWalkSpeed` 270.0 _charactermovement)))

(event `InputAction|ADS`
  (params (Key :type "Key Structure"))
  (bind _charactermovement (`self.CharacterMovement`))
  (bind _followcamera (`self.FollowCamera`))
  ;[1 1 1] ADS
  (:`Pressed`
    (set `self.IsADS` true)
    (set `CharacterMovementComponent.MaxWalkSpeed` 170.0 _charactermovement)
    (`CameraComponent.SetFieldOfView` _followcamera 70.0))
  (:`Released`
    (set `self.IsADS` false)
    (set `CharacterMovementComponent.MaxWalkSpeed` 270.0 _charactermovement)
    (`CameraComponent.SetFieldOfView` _followcamera 90.0)))

(fn `UserConstructionScript`)