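; Post-process actor that plays a tint and film grain flash when the player respawns.
; RespawnAtCheckpoint starts it, and Tick sweeps Timer rapidly down then back up, lerping the PostProcess component's settings in and out.
; SanityRespawn also respawns the player through BP_Respawner.
; The sanity countdown driving chromatic, bloom, dirt mask and grain, which calls SanityRespawn at zero, is disconnected and never runs, leaving ResetTimer without effect.
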(event `RespawnAtCheckpoint`
  ;[1 0.4892 0.5091] Events
  (set `self.RespawnPlayer` true)
  (set `self.CurrentValue` 0.0)
  (set `self.Timer` (`self.MaxTime`)))

(event `self.ReceiveBeginPlay`
  ;[1 0.4892 0.5091] Events
  (set `self.Timer` (`self.MaxTime`)))

(event `Reset Timer`
  ;[1 0.4892 0.5091] Events
  (set `self.ResetTimer` true))

(event `self.ReceiveTick`
  (params (DeltaSeconds :type "Float (single-precision)"))
  (bind _returnvalue (`KismetMathLibrary.Lerp` 0.0 (`self.RespawnEffectMaxValue`) (`self.CurrentValue`)))
  ;[1 0.4187 0.9394] Sanity Effect
  (set `self.DeltaSeconds` DeltaSeconds)
  (if (`self.RespawnPlayer`)
    (if (`self.Flip`)
      (set `self.Timer` (+ (`self.Timer`) (* (`self.DeltaSeconds`) 150.0)))
      (if (> (`self.Timer`) (`self.MaxTime`))
        (set `self.RespawnPlayer` false)
        (set `self.Flip` false)
        (else
          (set `self.CurrentValue` (/ (- (`self.MaxTime`) (`self.Timer`)) (`self.MaxTime`)) :!label _label)
          (bind _output_get (set `self.PostProcessSettings` (make `PostProcessSettings` :`WhiteTint` _returnvalue :`FilmGrainIntensity` _returnvalue)))
          (set `PostProcessComponent.Settings` _output_get (`self.PostProcess`))))
      (else
        (set `self.Timer` (- (`self.Timer`) (* (`self.DeltaSeconds`) 150.0)))
        (if (< (`self.Timer`) 0.0)
          (set `self.Flip` true)
          (else
            (goto _label)))))))

(event `SanityRespawn`
  ;[1 0.4892 0.5091] Events
  (bind _returnvalue (`GameplayStatics.GetActorOfClass` "/Game/_Game/Interactables/BP_Respawner.BP_Respawner_C"))
  (`/Game/_Game/Interactables/BP_Respawner.Respawn` _returnvalue (`GameplayStatics.GetPlayerPawn` 0))
  (set `self.RespawnPlayer` true)
  (set `self.ResetTimer` true))

(fn `UserConstructionScript`)