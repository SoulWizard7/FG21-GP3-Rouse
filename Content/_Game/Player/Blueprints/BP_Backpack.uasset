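; BP_Backpack is the player's backpack, with a widget that displays Freeze, Levitate and Sticky state from the character's ammo component.
; On BeginPlay it caches its UMG_Backpack widget and the BP_T7Character controlled by player 0.
; Every Tick it polls the AmmoComponent's three Effected values and pushes them into the widget's setters, with no event-driven updates.
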(event `self.ReceiveBeginPlay`
  (bind _asumg_backpack (cast `/Game/_Game/UI/Widgets/UMG_Backpack` (`WidgetComponent.GetUserWidgetObject` (`self.Widget`))))
  (set `self.WidgetRef` _asumg_backpack)
  (bind _asbp_t7character (cast `/Game/_Game/Player/ThirdPersonTest/BP_T7Character` (`GameplayStatics.GetPlayerPawn` 0)))
  (set `self.CharacterRef` _asbp_t7character))

(event `self.ReceiveTick`
  (params (DeltaSeconds :type "Float (single-precision)"))
  (bind _widgetref (`self.WidgetRef`))
  (`/Game/_Game/UI/Widgets/UMG_Backpack.SetFreeze` _widgetref (`T7AmmoComponent.EffectedFreeze` (`T7Character.AmmoComponent` (`self.CharacterRef`))))
  (`/Game/_Game/UI/Widgets/UMG_Backpack.SetLevitate` _widgetref (`T7AmmoComponent.EffectedLevitate` (`T7Character.AmmoComponent` (`self.CharacterRef`))))
  (`/Game/_Game/UI/Widgets/UMG_Backpack.SetSticky` _widgetref (`T7AmmoComponent.EffectedSticky` (`T7Character.AmmoComponent` (`self.CharacterRef`)))))

(fn `UserConstructionScript`)