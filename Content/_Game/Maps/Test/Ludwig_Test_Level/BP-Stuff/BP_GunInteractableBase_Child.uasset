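; Test-level child of BP_GunInteractableBase that makes a gun-interactable object react to acid.
; Overlapping an actor tagged Acid stops the inherited freeze, levitate and sticky behaviours and sets the Cube's collision to OverlapAll, so it no longer blocks.
; A custom Wah event stops the same three behaviours and destroys the actor; nothing in this graph calls it.
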(event `self.ReceiveBeginPlay`
  (`parent.ReceiveBeginPlay`))

(event `self.ReceiveActorBeginOverlap`
  (params (OtherActor :type "Actor Object Reference"))
  (if (`self.ActorHasTag` OtherActor "Acid")
    (`self.StopFreezeBehaviour`)
    (`self.StopLevitateBehaviour`)
    (`self.StopStickyBehaviour`)
    (`PrimitiveComponent.SetCollisionProfileName` (`self.Cube`) "OverlapAll" true)))

(event `/Game/_Game/Maps/Test/Ludwig_Test_Level/BP-Stuff/Int-Wah.Wah`
  (`self.StopFreezeBehaviour`)
  (`self.StopLevitateBehaviour`)
  (`self.StopStickyBehaviour`)
  (`self.K2_DestroyActor`))

(fn `UserConstructionScript`
  (`parent.UserConstructionScript`))