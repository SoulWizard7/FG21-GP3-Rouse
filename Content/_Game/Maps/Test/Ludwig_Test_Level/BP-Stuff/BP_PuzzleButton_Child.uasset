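; Puzzle button child Blueprint in a test level that acts as a pressure switch for actors tagged "Cube".
; Box collision begin and end overlaps call Activated or Deactivated, then fire the matching trigger on T7Interactable.
; Those events print debug text and set the BaseColor material's Color parameter to green when down and red when up.
; It does not count overlaps, so any tagged actor leaving deactivates it.
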(event `Activated`
  (`KismetSystemLibrary.PrintString` "Button down")
  (`MaterialInstanceDynamic.SetVectorParameterValue` (`self.BaseColor`) "Color" (struct :`G` 1.0 :`A` 1.0)))

(event `Deactivated`
  (`KismetSystemLibrary.PrintString` "Button up")
  (`MaterialInstanceDynamic.SetVectorParameterValue` (`self.BaseColor`) "Color" (struct :`R` 1.0 :`A` 1.0)))

(event `self.BoxCollision.OnComponentBeginOverlap`
  (params (OverlappedComponent :type "PrimitiveComponent Object Reference") (OtherActor :type "Actor Object Reference") (OtherComp :type "PrimitiveComponent Object Reference") (OtherBodyIndex :type Integer) (bFromSweep :type Boolean) (SweepResult :type "HitResult Structure (by ref)"))
  (if (`self.ActorHasTag` OtherActor "Cube")
    (`self.Activated`)
    (`T7InteractableComponent.TriggerActivate` (`self.T7Interactable`))))

(event `self.BoxCollision.OnComponentEndOverlap`
  (params (OverlappedComponent :type "PrimitiveComponent Object Reference") (OtherActor :type "Actor Object Reference") (OtherComp :type "PrimitiveComponent Object Reference") (OtherBodyIndex :type Integer))
  (if (`self.ActorHasTag` OtherActor "Cube")
    (`self.Deactivated`)
    (`T7InteractableComponent.TriggerDeactivate` (`self.T7Interactable`))))

(fn `UserConstructionScript`
  (`parent.UserConstructionScript`))