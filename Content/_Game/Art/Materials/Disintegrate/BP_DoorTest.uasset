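; BP_DoorTest is a test plank door that disintegrates when activated through T7InteractableResponse.
; Activation creates dynamic disintegration material instances on two mesh slots, plays a timeline driving their "Amount" parameter, and disables collision.
; Deactivation, gated by DoDeactivate, reverses the timeline and restores query and physics collision.
; Collision toggles right after the timeline starts, without waiting for the effect to finish.
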(event `self.T7InteractableResponse.OnActivate`
  (bind _plank_door (`self.plank_Door`))
  (bind _returnvalue (`PrimitiveComponent.CreateDynamicMaterialInstance` _plank_door 0 "/Game/_Game/Art/Materials/Disintegrate/Wood_MaterialDisint_Inst.Wood_MaterialDisint_Inst" "None"))
  (bind _returnvalue_2 (`PrimitiveComponent.CreateDynamicMaterialInstance` _plank_door 1 "/Game/_Game/Art/Materials/Disintegrate/Wood_MaterialDisint_Inst.Wood_MaterialDisint_Inst" "None"))
  (`|ExecutionSequence`
    (:`then_0`
      (bind (_direction _newtrack_0) (`Timeline|Timeline_0` :!label _label)
        (:`Update`
          (`MaterialInstanceDynamic.SetScalarParameterValue` _returnvalue "Amount" _newtrack_0)
          (`MaterialInstanceDynamic.SetScalarParameterValue` _returnvalue_2 "Amount" _newtrack_0))))
    (:`then_1`
      (`PrimitiveComponent.SetCollisionEnabled` (`self.plank_Door`) "NoCollision"))))

(event `self.T7InteractableResponse.OnDeactivate`
  (if (`self.DoDeactivate`)
    (`|ExecutionSequence`
      (:`then_0`
        (goto _label :!via `Reverse`))
      (:`then_1`
        (`PrimitiveComponent.SetCollisionEnabled` (`self.plank_Door`) "QueryAndPhysics")))))

(fn `UserConstructionScript`)