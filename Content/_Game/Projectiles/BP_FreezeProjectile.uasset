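; BP_FreezeProjectile is a freeze projectile that moves via T7ProjectileMovement on its sphere component.
; It spawns an unattached Niagara trail and moves it to the projectile's location every tick.
; A regular hit plays freeze sound and effects and calls AddAmmo on the player's BP_T7Character, while a no-response hit shows only its own effect.
; Both hits destroy the projectile and trail.
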(event `self.ReceiveBeginPlay`
  (`T7ProjectileMovementComponent.SetPrimitiveComponent` (`self.T7ProjectileMovement`) (`self.SphereComponent`))
  (bind _returnvalue (`NiagaraFunctionLibrary.SpawnSystemAtLocation` "/Game/_Game/Interactables/Gun/NS_FreezeProjectileTrail.NS_FreezeProjectileTrail" (`self.K2_GetActorLocation`)))
  (set `self.NiagaraActor` _returnvalue))

(event `self.ReceiveTick`
  (params (DeltaSeconds :type "Float (single-precision)"))
  (bind _niagaraactor (`self.NiagaraActor`)
    (:`then`
      (`SceneComponent.K2_SetWorldLocation` _niagaraactor (`self.K2_GetActorLocation`) false false))
    (:`else`)))

(event `self.ProjectileHit`
  (bind _returnvalue_location (`KismetMathLibrary.BreakTransform` (`self.GetTransform`)))
  (`GameplayStatics.PlaySoundAtLocation` "/Game/_Game/Sounds/Gun/Freeze/Sou_Freeze_Hit.Sou_Freeze_Hit" _returnvalue_location (struct) 0.8 1.0 0.0 "/Game/_Game/Art/Sound/SoundAttenuations/SA_HitDistance.SA_HitDistance" null null null)
  (`NiagaraFunctionLibrary.SpawnSystemAtLocation` "/Game/_Game/Projectiles/NS_FreezeHitEffect.NS_FreezeHitEffect" _returnvalue_location)
  (bind _asbp_t7character (cast `/Game/_Game/Player/ThirdPersonTest/BP_T7Character` (`GameplayStatics.GetPlayerPawn` 0))
    (:`then`
      (`/Game/_Game/Player/ThirdPersonTest/BP_T7Character.AddAmmo` _asbp_t7character))
    (:`CastFailed`
      _))
  (`self.K2_DestroyActor` :!label _label)
  (`ActorComponent.K2_DestroyComponent` (`self.NiagaraActor`)))

(event `self.ProjectileHitNoHitResponse`
  (bind _returnvalue_location (`KismetMathLibrary.BreakTransform` (`self.GetTransform`)))
  (`NiagaraFunctionLibrary.SpawnSystemAtLocation` "/Game/_Game/Projectiles/NS_NoResponseHitEffect.NS_NoResponseHitEffect" _returnvalue_location)
  (goto _label))

(fn `UserConstructionScript`)