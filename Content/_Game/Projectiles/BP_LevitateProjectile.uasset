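; BP_LevitateProjectile is the levitate projectile, moved by a T7ProjectileMovement component driving its sphere component.
; A separately spawned Niagara trail follows it every tick.
; A hit plays an impact sound and levitation effect, then calls AddAmmo on the player character.
; A no-response hit shows a different effect without adding ammo; both outcomes destroy the projectile and trail.
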(event `self.ReceiveBeginPlay`
  (`T7ProjectileMovementComponent.SetPrimitiveComponent` (`self.T7ProjectileMovement`) (`self.SphereComponent`))
  (bind _returnvalue (`NiagaraFunctionLibrary.SpawnSystemAtLocation` "/Game/_Game/Interactables/Gun/NS_LevitateProjectileTrail.NS_LevitateProjectileTrail" (`self.K2_GetActorLocation`) (struct) (1.0 1.0 1.0) false))
  (set `self.NiagaraComponent` _returnvalue))

(event `self.ReceiveTick`
  (params (DeltaSeconds :type "Float (single-precision)"))
  (bind _niagaracomponent (`self.NiagaraComponent`)
    (:`then`
      (`SceneComponent.K2_SetWorldLocation` _niagaracomponent (`self.K2_GetActorLocation`) false false))
    (:`else`)))

(event `self.ProjectileHit`
  (bind _returnvalue_location (`KismetMathLibrary.BreakTransform` (`self.GetTransform`)))
  (`GameplayStatics.PlaySoundAtLocation` "/Game/_Game/Sounds/Gun/Levitate/Float_impact.Float_impact" _returnvalue_location (struct) 0.8 1.0 0.0 "/Game/_Game/Art/Sound/SoundAttenuations/SA_HitDistance.SA_HitDistance" null null null)
  (`NiagaraFunctionLibrary.SpawnSystemAtLocation` "/Game/_Game/Projectiles/NS_LevitationHitEffect.NS_LevitationHitEffect" _returnvalue_location)
  (bind _asbp_t7character (cast `/Game/_Game/Player/ThirdPersonTest/BP_T7Character` (`GameplayStatics.GetPlayerPawn` 0))
    (:`then`
      (`/Game/_Game/Player/ThirdPersonTest/BP_T7Character.AddAmmo` _asbp_t7character)
      (`self.K2_DestroyActor`)
      (`ActorComponent.K2_DestroyComponent` (`self.NiagaraComponent`)))
    (:`CastFailed`
      (`self.K2_DestroyActor` :!label _label)
      (`ActorComponent.K2_DestroyComponent` (`self.NiagaraComponent`)))))

(event `self.ProjectileHitNoHitResponse`
  (bind _returnvalue_location (`KismetMathLibrary.BreakTransform` (`self.GetTransform`)))
  (`NiagaraFunctionLibrary.SpawnSystemAtLocation` "/Game/_Game/Projectiles/NS_NoResponseHitEffect.NS_NoResponseHitEffect" _returnvalue_location)
  (goto _label))

(fn `UserConstructionScript`)