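; Test actor that aims a ballistic launch from Origin to Target through a set apex height, previewing it with debug lines.
; Each tick, or on a construction-script editor timer when Gizmos is on, it derives range, launch angle and impulse, then pitches Origin relative to the aim line.
; ShootProjectile spawns BP_ProjectileTest with gravity adjusted to the aim's up vector and applies the impulse.
; Actors overlapping Collision are destroyed.
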(event `self.ReceiveTick`
  (params (DeltaSeconds :type "Float (single-precision)"))
  (`self.CalculateRange`)
  (`self.CalculateAngle`)
  (`self.CalculateForce`)
  (`self.Debugging`))

(event `self.Collision.OnComponentBeginOverlap`
  (params (OverlappedComponent :type "PrimitiveComponent Object Reference") (OtherActor :type "Actor Object Reference") (OtherComp :type "PrimitiveComponent Object Reference") (OtherBodyIndex :type Integer) (bFromSweep :type Boolean) (SweepResult :type "HitResult Structure (by ref)"))
  (`self.K2_DestroyActor` OtherActor))

(fn `CalculateAngle`
  (returns (Angle :type "Float (double-precision)"))
  (bind _output_get (set `self.Angle` (`T7PhysicsBlueprintLibrary.GetAngleDegrees` (`self.Range`) (`self.Height`))))
  (`SceneComponent.K2_SetWorldRotation` (`self.Origin`) (`KismetMathLibrary.MakeRotator` 0.0 _output_get) false false)
  (return _output_get))

(fn `CalculateForce`
  (returns (Force :type "Float (double-precision)"))
  (bind _output_get (set `self.ForceMagnitude` (`T7PhysicsBlueprintLibrary.GetImpulseFromDegrees` (`self.Height`) (`self.Angle`))))
  (return _output_get))

(fn `CalculateRange`
  (returns (ReturnValue :type "Float (double-precision)"))
  (bind _output_get (set `self.Range` (`KismetMathLibrary.Vector_Distance` (`SceneComponent.K2_GetComponentLocation` (`self.Origin`)) (`SceneComponent.K2_GetComponentLocation` (`self.Target`)))))
  (return _output_get))

(fn `Debugging`
  (bind _aimarrow (`self.AimArrow`))
  (bind _returnvalue (`SceneComponent.K2_GetComponentLocation` (`self.Target`)))
  (bind _returnvalue_2 (`KismetMathLibrary.Normal` (`self.GetAimVector`)))
  (bind _returnvalue_3 (+ (* (`SceneComponent.GetForwardVector` _aimarrow) (/ (`self.Range`) 2.0)) (`SceneComponent.K2_GetComponentLocation` _aimarrow)))
  (`KismetSystemLibrary.DrawDebugLine` (`SceneComponent.K2_GetComponentLocation` (`self.Origin`)) _returnvalue (struct :`R` 1.0 :`A` 1.0) 0.1 3.0)
  (`KismetSystemLibrary.DrawDebugSphere` _returnvalue 20.0 12 (struct :`G` 1.0 :`A` 1.0) 0.1 1.0)
  (`SceneComponent.K2_SetWorldRotation` (`self.AimArrow`) (`KismetMathLibrary.Conv_VectorToRotator` _returnvalue_2) false false)
  (`SceneComponent.K2_SetWorldRotation` (`self.Origin`) (`KismetMathLibrary.Conv_VectorToRotator` (`KismetMathLibrary.RotateAngleAxis` _returnvalue_2 (`self.Angle`) (`KismetMathLibrary.NegateVector` (`SceneComponent.GetRightVector` (`self.AimArrow`))))) false false)
  (`KismetSystemLibrary.DrawDebugLine` _returnvalue_3 (+ _returnvalue_3 (* (`SceneComponent.GetUpVector` (`self.AimArrow`)) (`self.Height`))) (struct :`B` 1.0 :`A` 1.0) 0.1 3.0))

(fn `EditorTick`
  (`self.CalculateRange`)
  (`self.CalculateAngle`)
  (`self.CalculateForce`)
  (`self.Debugging`))

(fn `GetAimVector`
  (returns (ReturnValue :type "Vector Structure"))
  (return (- (`SceneComponent.K2_GetComponentLocation` (`self.Target`)) (`SceneComponent.K2_GetComponentLocation` (`self.Origin`)))))

(fn `ShootProjectile`
  (bind _returnvalue (`|SpawnActorFromClass` "/Game/_Game/Projectiles/Trajectory/BP_ProjectileTest.BP_ProjectileTest_C" (`SceneComponent.K2_GetComponentToWorld` (`self.Origin`)) "AlwaysSpawn" "OverrideRootScale" null null))
  (set `/Game/_Game/Projectiles/Trajectory/BP_ProjectileTest.GravityForce` (`T7PhysicsBlueprintLibrary.GetAdjustedGravity` (`SceneComponent.GetUpVector` (`self.AimArrow`))) _returnvalue)
  (`PrimitiveComponent.AddImpulse` (`/Game/_Game/Projectiles/Trajectory/BP_ProjectileTest.Sphere` _returnvalue) (* (`SceneComponent.GetForwardVector` (`self.Origin`)) (`self.ForceMagnitude`)) "None" false))

(fn `UserConstructionScript`
  (if (`self.Gizmos`)
    (`KismetSystemLibrary.K2_SetTimer` null "EditorTick" 0.01 true)))