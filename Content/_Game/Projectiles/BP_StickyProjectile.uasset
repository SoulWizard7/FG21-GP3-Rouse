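; BP_StickyProjectile is a sticky projectile moved by T7ProjectileMovement on its sphere component, with a Niagara trail that follows it every tick.
; A normal hit plays the sticky sound and effect, then calls AddAmmo on the player's BP_T7Character.
; A no-response hit spawns only its own effect.
; Both hit paths set the Hit flag and destroy the projectile and trail.
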(event `self.ReceiveBeginPlay`
  (`T7ProjectileMovementComponent.SetPrimitiveComponent` (`self.T7ProjectileMovement`) (`self.SphereComponent`))
  (bind _returnvalue (`NiagaraFunctionLibrary.SpawnSystemAtLocation` "/Game/_Game/Interactables/Gun/NS_StickyProjectileTrail.NS_StickyProjectileTrail" (`self.K2_GetActorLocation`)))
  (set `self.Niagara Component` _returnvalue))

(event `self.ReceiveTick`
  (params (DeltaSeconds :type "Float (single-precision)"))
  (bind _niagara_component (`self.Niagara Component`)
    (:`then`
      (`SceneComponent.K2_SetWorldLocation` _niagara_component (`self.K2_GetActorLocation`) false false))
    (:`else`)))

(event `self.ProjectileHit`
  (bind _returnvalue_location (`KismetMathLibrary.BreakTransform` (`self.GetTransform`)))
  (set `self.Hit` true)
  (`GameplayStatics.PlaySoundAtLocation` "/Game/_Game/Sounds/Gun/Slime/Sou_Sticky_Hit.Sou_Sticky_Hit" _returnvalue_location (struct) 0.8 1.0 0.0 "/Game/_Game/Art/Sound/SoundAttenuations/SA_HitDistance.SA_HitDistance" null null null)
  (`NiagaraFunctionLibrary.SpawnSystemAtLocation` "/Game/_Game/Projectiles/NS_StickyHitEffect.NS_StickyHitEffect" _returnvalue_location)
  (bind _asbp_t7character (cast `/Game/_Game/Player/ThirdPersonTest/BP_T7Character` (`GameplayStatics.GetPlayerPawn` 0))
    (:`then`
      (`/Game/_Game/Player/ThirdPersonTest/BP_T7Character.AddAmmo` _asbp_t7character))
    (:`CastFailed`
      _))
  (`self.K2_DestroyActor` :!label _label)
  (`ActorComponent.K2_DestroyComponent` (`self.Niagara Component`)))

(event `self.ProjectileHitNoHitResponse`
  (bind _returnvalue_location (`KismetMathLibrary.BreakTransform` (`self.GetTransform`)))
  (set `self.Hit` true)
  (`NiagaraFunctionLibrary.SpawnSystemAtLocation` "/Game/_Game/Projectiles/NS_NoResponseHitEffect.NS_NoResponseHitEffect" _returnvalue_location)
  (goto _label))

(fn `UserConstructionScript`)