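; One-shot checkpoint actor that sets the player's respawn point when the player overlaps its box.
; It stores its respawn transform on BP_T7Character, notifies the character, retracts ammo from every BP_GunInteractableBase and replenishes the player's ammo.
; Activation clears IsActivated, plays sounds, brightens the point light, raises the pivot via a timeline and sets the lamp's dynamic-material emissive.
; The look-at-player rotation is disconnected.
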(event `self.ReceiveBeginPlay`
  (set `self.RespawnTransform` (`SceneComponent.K2_GetComponentToWorld` (`self.RespawnTransformPosition`)))
  (bind _returnvalue (`PrimitiveComponent.CreateDynamicMaterialInstance` (`self.StaticMesh`) 0 "/Game/_Game/Art/ArtTest_F/Lamp/M_CheckpointLamp.M_CheckpointLamp" "None"))
  (set `self.MaterialRef` _returnvalue))

(event `self.Box.OnComponentBeginOverlap`
  (params (OverlappedComponent :type "PrimitiveComponent Object Reference") (OtherActor :type "Actor Object Reference") (OtherComp :type "PrimitiveComponent Object Reference") (OtherBodyIndex :type Integer) (bFromSweep :type Boolean) (SweepResult :type "HitResult Structure (by ref)"))
  (bind _returnvalue (`GameplayStatics.GetPlayerPawn` 0))
  (bind _returnvalue_2 (`self.K2_GetActorLocation`))
  ;[1 0.7827 0.3277] Checkpoint
  (if (`self.IsActivated`)
    (if (== OtherActor _returnvalue)
      (`KismetSystemLibrary.PrintString` "CheckPoint Hit Player")
      (bind _asbp_t7character (cast `/Game/_Game/Player/ThirdPersonTest/BP_T7Character` _returnvalue))
      (bind _output_get (set `self.CharacterRef` _asbp_t7character))
      (set `/Game/_Game/Player/ThirdPersonTest/BP_T7Character.RespawnTransformPosition` (`self.RespawnTransform`) _output_get)
      (`/Game/_Game/Player/ThirdPersonTest/BP_T7Character.EnteredCheckpoint` _asbp_t7character)
      (`self.Remove powers from all blocks`)
      (set `self.IsActivated` false)
      (`GameplayStatics.PlaySoundAtLocation` "/Game/_Game/Sounds/SFX/SFX/S_Checkpoint.S_Checkpoint" _returnvalue_2 (struct) 1.0 1.0 0.0 null null null null)
      (`GameplayStatics.PlaySoundAtLocation` "/Game/_Game/Sound_Cue/Sc_UIButtonClick.Sc_UIButtonClick" _returnvalue_2 (struct) 0.6 1.0 0.0 null null null null)
      (`LightComponent.SetIntensity` (`self.PointLight`) 100.0)
      (bind (_direction _alpha) (`Timeline|JumpAnim` :!via `PlayFromStart`)
        (:`Update`
          (`SceneComponent.K2_SetRelativeLocation` (`self.Pivot`) (`KismetMathLibrary.MakeVector` 0.0 0.0 (* _alpha 15.0)) false false)
          (`MaterialInstanceDynamic.SetScalarParameterValue` (`self.MaterialRef`) "Emissive Power" 0.5))))))

(event `Remove powers from all blocks`
  ;[1 0.2864 0.9561] Remove powers from all blocks and replenish ammo
  (bind _outactors (`GameplayStatics.GetAllActorsOfClass` "/Game/_Game/Interactables/Gun/BP_GunInteractableBase.BP_GunInteractableBase_C"))
  (for _array_element _outactors
    (`/Game/_Game/Interactables/Gun/BP_GunInteractableBase.RetractAmmo` _array_element))
  (`KismetSystemLibrary.PrintString` "stop all powers" true true (struct :`R` 1.0 :`G` 0.905882 :`A` 1.0))
  (bind _asbp_t7character (cast `/Game/_Game/Player/ThirdPersonTest/BP_T7Character` (`GameplayStatics.GetPlayerPawn` 0)))
  (`T7AmmoComponent.ReplenishAmmo` (`T7Character.AmmoComponent` _asbp_t7character))
  (`KismetSystemLibrary.PrintString` "Ammo replenished" true true (struct :`R` 1.0 :`G` 0.905882 :`A` 1.0)))

(event `self.ReceiveTick`
  (params (DeltaSeconds :type "Float (single-precision)"))
  ;[1 1 1] Deprecated
)

(fn `UserConstructionScript`)