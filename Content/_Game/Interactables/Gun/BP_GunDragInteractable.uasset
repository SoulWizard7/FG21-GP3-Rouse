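; BP_GunDragInteractable is a gun-related drag interactable whose box is handled by a PushableComponent.
; On BeginPlay it passes its BoxComponent to the PushableComponent.
; The construction script draws a downward debug line showing that component's ground trace length.
; Every Tick runs debug output, printing the component's grounded state and drawing a sphere offset from the actor along BoxSide.
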(event `self.ReceiveBeginPlay`
  (set `T7PushableComponent.BoxComponent` (`self.BoxComponent`) (`self.PushableComponent`)))

(event `self.ReceiveTick`
  (params (DeltaSeconds :type "Float (single-precision)"))
  (`self.Debugging`))

(fn `Debugging`
  (`KismetSystemLibrary.PrintString` (`KismetStringLibrary.Conv_BoolToString` (`T7PushableComponent.bIsGrounded` (`self.PushableComponent`))) true false (struct :`G` 0.66 :`B` 1.0 :`A` 1.0) 0.0)
  (`KismetSystemLibrary.DrawDebugSphere` (+ (`self.K2_GetActorLocation`) (* (`self.BoxSide`) 80.0)) 20.0 12 (struct :`R` 1.0 :`A` 1.0) 0.0 2.0))

(fn `UserConstructionScript`
  (bind _returnvalue (`self.K2_GetActorLocation`))
  (`KismetSystemLibrary.DrawDebugLine` _returnvalue (+ _returnvalue (* (`KismetMathLibrary.Vector_Down`) (`T7PushableComponent.GroundTraceLength` (`self.PushableComponent`)))) (struct :`R` 1.0 :`A` 1.0) 1.0 10.0))