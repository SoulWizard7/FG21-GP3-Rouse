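; Test base actor for a gun interactable cube that reacts to levitate, freeze, sticky and trace-hit response components.
; Each state tints a dynamic material; starting freeze or sticky stops the other states, as does stopping levitate.
; Tick pushes the cube upward with gravity off while levitating, or pins the actor to its saved sticky position.
; Freeze only changes color here, and the sticky overlap check's result is ignored.
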(event `self.ReceiveBeginPlay`
  (bind _returnvalue (`PrimitiveComponent.CreateDynamicMaterialInstance` (`self.Cube`) 0 "/Game/_Game/Interactables/Gun/Materials/M_GunInteractable.M_GunInteractable" "None"))
  (bind _output_get (set `self.MaterialRef` _returnvalue))
  (`MaterialInstanceDynamic.SetVectorParameterValue` _output_get "Color" (struct :`R` 1.0 :`G` 1.0 :`B` 1.0 :`A` 1.0)))

(event `self.ReceiveTick`
  (params (DeltaSeconds :type "Float (single-precision)"))
  (set `self.DeltaSeconds` DeltaSeconds)
  ;[1 1 1] Levitation Behaviour
  (if (`T7LevitateResponse.bIsLevitating` (`self.T7LevitateResponse`))
    (`PrimitiveComponent.AddForce` (`self.Cube`) (* (`KismetMathLibrary.Vector_Up`) (`self.LevitateForce`)) "None" false)
    (else
      ;[1 1 1] StickyBehaviour
      (if (`T7StickyResponse.bIsSticky` (`self.T7StickyResponse`))
        (`KismetSystemLibrary.PrintString` "isSticky = true" true true (struct :`R` 1.0 :`G` 0.141462 :`B` 0.919605 :`A` 1.0) 1.0)
        (`self.K2_SetActorLocation` (`self.StickyPosition`))))))

(event `self.T7LevitateResponse.OnStartLevitate`
  ;[1 1 1] Levitate
  (`PrimitiveComponent.SetEnableGravity` (`self.Cube`) false)
  (`MaterialInstanceDynamic.SetVectorParameterValue` (`self.MaterialRef`) "Color" (struct :`R` 0.29228 :`G` 1.0 :`B` 0.441067 :`A` 1.0)))

(event `self.T7LevitateResponse.OnStopLevitate`
  ;[1 1 1] Levitate
  (`T7FreezeResponse.StopFreeze` (`self.T7FreezeResponse`))
  (`T7StickyResponse.StopSticky` (`self.T7StickyResponse`))
  (`MaterialInstanceDynamic.SetVectorParameterValue` (`self.MaterialRef`) "Color" (struct :`R` 1.0 :`G` 1.0 :`B` 1.0 :`A` 1.0))
  (`PrimitiveComponent.SetEnableGravity` (`self.Cube`) true))

(event `self.T7FreezeResponse.OnStartFreeze`
  ;[1 1 1] Freezing
  (`T7LevitateResponse.StopLevitate` (`self.T7LevitateResponse`))
  (`T7StickyResponse.StopSticky` (`self.T7StickyResponse`))
  (`MaterialInstanceDynamic.SetVectorParameterValue` (`self.MaterialRef`) "Color" (struct :`G` 0.165959 :`B` 1.0 :`A` 1.0)))

(event `self.T7FreezeResponse.OnStopFreeze`
  ;[1 1 1] Freezing
  (`MaterialInstanceDynamic.SetVectorParameterValue` (`self.MaterialRef`) "Color" (struct :`R` 1.0 :`G` 1.0 :`B` 1.0 :`A` 1.0)))

(event `self.T7StickyResponse.OnStartSticky`
  ;[1 1 1] Sticky
  (`T7LevitateResponse.StopLevitate` (`self.T7LevitateResponse`))
  (`T7FreezeResponse.StopFreeze` (`self.T7FreezeResponse`))
  (`MaterialInstanceDynamic.SetVectorParameterValue` (`self.MaterialRef`) "Color" (struct :`R` 1.0 :`G` 0.537518 :`B` 0.072917 :`A` 1.0))
  (`KismetSystemLibrary.BoxOverlapActors` (`SceneComponent.K2_GetComponentLocation` (`self.Cube`)) (`self.StickyBoxExtent`) (`|MakeArray` "ObjectTypeQuery1" :!type "EObjectTypeQuery Enum"))
  (if true
    (set `self.StickyPosition` (`SceneComponent.K2_GetComponentLocation` (`self.Cube`)))))

(event `self.T7StickyResponse.OnStopSticky`
  ;[1 1 1] Sticky
  (`MaterialInstanceDynamic.SetVectorParameterValue` (`self.MaterialRef`) "Color" (struct :`R` 1.0 :`G` 1.0 :`B` 1.0 :`A` 1.0)))

(event `self.T7TraceHitResponse.OnHitEnter`
  ;[1 1 1] Trace hit
  (`KismetSystemLibrary.PrintString` "Hit enter")
  (`MaterialInstanceDynamic.SetVectorParameterValue` (`self.MaterialRef`) "Color" (struct :`G` 1.0 :`A` 1.0)))

(event `self.T7TraceHitResponse.OnHitExit`
  ;[1 1 1] Trace hit
  (`KismetSystemLibrary.PrintString` "Hit exit")
  (`MaterialInstanceDynamic.SetVectorParameterValue` (`self.MaterialRef`) "Color" (struct :`R` 1.0 :`G` 1.0 :`B` 1.0 :`A` 1.0)))

(event `self.T7TraceHitResponse.OnInteract`
  ;[1 1 1] Trace hit
  (`KismetSystemLibrary.PrintString` "Interact"))

(fn `UserConstructionScript`)