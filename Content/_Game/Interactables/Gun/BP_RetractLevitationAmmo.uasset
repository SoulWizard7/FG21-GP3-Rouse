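; BP_RetractLevitationAmmo is a levitation gun ammo actor with a Niagara effect that flies back to the player.
; A Tick timer stages the motion: a one-second drift along the sphere's up vector and toward the player, then a half-second pause.
; It then lerps from its current location to the player with a growing alpha, accelerating the homing.
; The actor destroys itself when its collider overlaps the player pawn.
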(event `self.ReceiveBeginPlay`
  (`ActorComponent.Activate` (`self.Niagara`) true))

(event `self.ReceiveTick`
  (params (DeltaSeconds :type "Float (single-precision)"))
  ;[1 0.4354 0.7883] Retract ammo movement system
  (bind _output_get (set `self.DeltaSecond` DeltaSeconds))
  (set `self.timer` (+ _output_get (`self.timer`)))
  (if (> (`self.timer`) 1.0)
    (if (> (`self.timer`) 1.5)
      (set `self.CurrentVector` (`self.K2_GetActorLocation`))
      (`self.K2_SetActorLocation` (`KismetMathLibrary.VLerp` (`self.CurrentVector`) (`self.K2_GetActorLocation` (`GameplayStatics.GetPlayerPawn` 0)) (/ (`self.MoveForwardLerpValue`) 2.0)))
      (set `self.MoveForwardLerpValue` (+ (`self.MoveForwardLerpValue`) (`self.DeltaSecond`))))
    (else
      (`self.K2_AddActorLocalOffset` (+ (* (`SceneComponent.GetUpVector` (`self.Sphere`)) (`self.MoveUpSpeed`)) (* (`KismetMathLibrary.Normal` (- (`self.K2_GetActorLocation` (`GameplayStatics.GetPlayerPawn` 0)) (`self.K2_GetActorLocation`))) (`self.MoveUpSpeed`)))))))

(event `self.Collider.OnComponentBeginOverlap`
  (params (OverlappedComponent :type "PrimitiveComponent Object Reference") (OtherActor :type "Actor Object Reference") (OtherComp :type "PrimitiveComponent Object Reference") (OtherBodyIndex :type Integer) (bFromSweep :type Boolean) (SweepResult :type "HitResult Structure (by ref)"))
  ;[1 0.4354 0.7883] Retract ammo movement system
  (if (== OtherActor (`GameplayStatics.GetPlayerPawn` 0))
    (`self.K2_DestroyActor`)))

(fn `UserConstructionScript`)