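; BP_PuzzleButtonLook is an interactable puzzle button that highlights while a trace hits it.
; BeginPlay creates a dynamic instance of M_GunInteractable on the Cube and sets its Color parameter to white.
; Events from the T7TraceHitResponse component turn the cube green on hit enter and back to white on hit exit.
; Interact only prints a debug string, with no puzzle logic attached.
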(event `self.ReceiveBeginPlay`
  (bind _returnvalue (`PrimitiveComponent.CreateDynamicMaterialInstance` (`self.Cube`) 0 "/Game/_Game/Interactables/Gun/Materials/M_GunInteractable.M_GunInteractable" "None"))
  (bind _output_get (set `self.MaterialRef` _returnvalue))
  (`MaterialInstanceDynamic.SetVectorParameterValue` _output_get "Color" (struct :`R` 1.0 :`G` 1.0 :`B` 1.0 :`A` 1.0)))

(event `self.T7TraceHitResponse.OnHitEnter`
  ;[1 1 1] Trace hit
  (`KismetSystemLibrary.PrintString` "Hit enter")
  (`MaterialInstanceDynamic.SetVectorParameterValue` (`self.MaterialRef`) "Color" (struct :`G` 1.0 :`A` 1.0)))

(event `self.T7TraceHitResponse.OnHitExit`
  ;[1 1 1] Trace hit
  (`KismetSystemLibrary.PrintString` "Hit exit")
  (`MaterialInstanceDynamic.SetVectorParameterValue` (`self.MaterialRef`) "Color" (struct :`R` 1.0 :`G` 1.0 :`B` 1.0 :`A` 1.0)))

(event `self.T7TraceHitResponse.OnInteract`
  ;[1 1 1] Trace hit
  (`KismetSystemLibrary.PrintString` "Interact"))

(fn `UserConstructionScript`)