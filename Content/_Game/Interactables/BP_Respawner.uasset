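; BP_Respawner is an overlap volume that sends the player back to their checkpoint and resets gun interactables that enter it.
; For the player, it triggers the sanity post-process respawn effect, runs the character's fall-to-void, then after a delay teleports to the stored respawn transform and resets every gun interactable.
; Other gun interactables are reset individually, except those in an ignore list, which only retract their ammo.
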(event `self.ReceiveBeginPlay`
  (bind _returnvalue (`GameplayStatics.GetActorOfClass` "/Game/_Game/PostProcess/BP_SanityPostProcess.BP_SanityPostProcess_C"))
  (set `self.PostProcessActor` _returnvalue))

(event `self.ReceiveActorBeginOverlap`
  (params (OtherActor :type "Actor Object Reference"))
  (`self.Respawn` OtherActor))

(event `Respawn`
  (params (`Other Actor` :type "Actor Object Reference"))
  (if (== `Other Actor` (`GameplayStatics.GetPlayerPawn` 0))
    (bind _asbp_t7character (cast `/Game/_Game/Player/ThirdPersonTest/BP_T7Character` `Other Actor`)
      (:`then`
        (`/Engine/EditorBlueprintResources/StandardMacros.IsValid` _asbp_t7character
          (:`Is Valid`
            (`/Game/_Game/PostProcess/BP_SanityPostProcess.RespawnAtCheckpoint` (`self.PostProcessActor`))
            (`KismetSystemLibrary.PrintString` "Respawn at checkpoint in BP_Respawner")
            (`/Game/_Game/Player/ThirdPersonTest/BP_T7Character.FallToVoid` _asbp_t7character)
            (`KismetSystemLibrary.Delay` 2.0)
            (bind (_respawntransformposition_location _respawntransformposition_rotation) (`KismetMathLibrary.BreakTransform` (`/Game/_Game/Player/ThirdPersonTest/BP_T7Character.RespawnTransformPosition` _asbp_t7character)))
            (`self.K2_TeleportTo` _asbp_t7character _respawntransformposition_location _respawntransformposition_rotation)
            (`/Game/_Game/Player/ThirdPersonTest/BP_T7Character.StopFallToVoid` _asbp_t7character)
            (bind _outactors (`GameplayStatics.GetAllActorsOfClass` "/Game/_Game/Interactables/Gun/BP_GunInteractableBase.BP_GunInteractableBase_C"))
            (for _array_element _outactors
              (`/Game/_Game/Interactables/Gun/BP_GunInteractableBase.ResetInteractable` _array_element)))))
      (:`CastFailed`
        (`KismetSystemLibrary.PrintString` "Respawner Cast failed")))
    (else
      (bind _asbp_gun_interactable_base (cast `/Game/_Game/Interactables/Gun/BP_GunInteractableBase` `Other Actor`))
      (if (not (`KismetArrayLibrary.Array_Contains` (`self.InteractableToIgnore`) _asbp_gun_interactable_base))
        (`/Game/_Game/Interactables/Gun/BP_GunInteractableBase.ResetInteractable` _asbp_gun_interactable_base)
        (else
          (`/Game/_Game/Interactables/Gun/BP_GunInteractableBase.RetractAmmo` _asbp_gun_interactable_base))))))

(fn `UserConstructionScript`)