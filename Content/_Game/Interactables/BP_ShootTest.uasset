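; BP_ShootTest is a debug interactable that tests the T7 Freeze, Sticky and Levitate response components.
; Each component's start event prints a message and immediately calls that component's stop function.
; Each stop event prints its own message, confirming the start and stop round trip.
; It has no other active logic.
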(event `self.T7FreezeResponse.OnStartFreeze`
  (`KismetSystemLibrary.PrintString` "Start freeze")
  (`T7FreezeResponse.StopFreeze` (`self.T7FreezeResponse`)))

(event `self.T7FreezeResponse.OnStopFreeze`
  (`KismetSystemLibrary.PrintString` "Stop Freeze"))

(event `self.T7StickyResponse.OnStartSticky`
  (`KismetSystemLibrary.PrintString` "Start Sticky")
  (`T7StickyResponse.StopSticky` (`self.T7StickyResponse`)))

(event `self.T7StickyResponse.OnStopSticky`
  (`KismetSystemLibrary.PrintString` "Stop Sticky"))

(event `self.T7LevitateResponse.OnStartLevitate`
  (`KismetSystemLibrary.PrintString` "Start Levitate")
  (`T7LevitateResponse.StopLevitate` (`self.T7LevitateResponse`)))

(event `self.T7LevitateResponse.OnStopLevitate`
  (`KismetSystemLibrary.PrintString` "Stop Levitate"))

(fn `UserConstructionScript`)