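; BP_PuzzleButton is a pressure-style puzzle button that stays pressed while actors carrying a T7InteractableTrigger component overlap its box.
; An overlap count drives activation and deactivation on its T7Interactable component and tells connected wires to switch color.
; Activation and deactivation recolor three dynamic materials between green and red, play a click sound, and run or reverse a timeline that pushes the model along Z.
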(event `self.ReceiveBeginPlay`
  (bind _returnvalue (`PrimitiveComponent.CreateDynamicMaterialInstance` (`self.Model`) 1 "/Game/_Game/Art/ArtTest_Marika/M_ButtonBase.M_ButtonBase" "None"))
  (set `self.BaseColor` _returnvalue)
  (bind _returnvalue_2 (`PrimitiveComponent.CreateDynamicMaterialInstance` (`self.Model`) 0 "/Game/_Game/Art/ArtTest_Marika/M_ButtonSides.M_ButtonSides" "None"))
  (set `self.OutsideColor` _returnvalue_2)
  (bind _returnvalue_3 (`PrimitiveComponent.CreateDynamicMaterialInstance` (`self.Model`) 2 "/Game/_Game/Art/ArtTest_Marika/M_ButtonInside.M_ButtonInside" "None"))
  (set `self.InsideColor` _returnvalue_3))

(event `self.T7Interactable.OnActivate`
  ;[1 1 1] Activate/Deactivate Events
  (`KismetSystemLibrary.PrintString` "Button down")
  (`MaterialInstanceDynamic.SetVectorParameterValue` (`self.BaseColor`) "Color" (struct :`R` 0.705638 :`G` 1.0 :`B` 0.244792 :`A` 1.0))
  (`MaterialInstanceDynamic.SetVectorParameterValue` (`self.OutsideColor`) "Color" (struct :`R` 0.396568 :`G` 0.552083 :`B` 0.152398 :`A` 1.0))
  (`MaterialInstanceDynamic.SetVectorParameterValue` (`self.InsideColor`) "Color" (struct :`R` 0.45369 :`G` 0.635417 :`B` 0.079427 :`A` 1.0))
  (`MaterialInstanceDynamic.SetVectorParameterValue` (`self.BaseColor`) "Emissive Color" (struct :`R` 0.489831 :`G` 0.640625 :`B` 0.103434 :`A` 1.0))
  (`GameplayStatics.PlaySoundAtLocation` "/Game/_Game/Sounds/Puzzle_Components/212737-button-on-off-029.212737-button-on-off-029" (`SceneComponent.K2_GetComponentLocation` (`self.DefaultSceneRoot`)) (struct) 1.0 1.0 0.0 null null null null)
  (bind (_direction _pushz) (`Timeline|PushAnim` :!label _label)
    (:`Update`
      (`SceneComponent.K2_SetRelativeLocation` (`self.Model`) (`KismetMathLibrary.MakeVector` 0.0 0.0 _pushz) false false))))

(event `self.T7Interactable.OnDeactivate`
  ;[1 1 1] Activate/Deactivate Events
  (`KismetSystemLibrary.PrintString` "Button up")
  (`MaterialInstanceDynamic.SetVectorParameterValue` (`self.BaseColor`) "Color" (struct :`R` 0.401978 :`G` 0.107023 :`B` 0.135633 :`A` 1.0))
  (`MaterialInstanceDynamic.SetVectorParameterValue` (`self.OutsideColor`) "Color" (struct :`R` 0.533277 :`G` 0.049707 :`B` 0.064803 :`A` 1.0))
  (`MaterialInstanceDynamic.SetVectorParameterValue` (`self.InsideColor`) "Color" (struct :`R` 0.23074 :`G` 0.028426 :`B` 0.035601 :`A` 1.0))
  (`MaterialInstanceDynamic.SetVectorParameterValue` (`self.BaseColor`) "Emissive Color" (struct :`R` 0.439657 :`G` 0.068478 :`B` 0.072272 :`A` 1.0))
  (`GameplayStatics.PlaySoundAtLocation` "/Game/_Game/Sounds/Puzzle_Components/212740-button-on-off-035.212740-button-on-off-035" (`SceneComponent.K2_GetComponentLocation` (`self.DefaultSceneRoot`)) (struct) 1.0 1.0 0.0 null null null null)
  (goto _label :!via `Reverse`))

(event `self.BoxCollision.OnComponentBeginOverlap`
  (params (OverlappedComponent :type "PrimitiveComponent Object Reference") (OtherActor :type "Actor Object Reference") (OtherComp :type "PrimitiveComponent Object Reference") (OtherBodyIndex :type Integer) (bFromSweep :type Boolean) (SweepResult :type "HitResult Structure (by ref)"))
  ;[1 1 1] Collision handling
  (`/Engine/EditorBlueprintResources/StandardMacros.IsValid` (`self.GetComponentByClass` OtherActor "/Script/GP3.T7InteractableTrigger")
    (:`Is Valid`
      (`/Engine/EditorBlueprintResources/StandardMacros.IncrementInt` (`self.OverlapCount`)
        (:`  `
          (if (not (`T7InteractableComponent.bIsActivated` (`self.T7Interactable`)))
            (`T7InteractableComponent.TriggerActivate` (`self.T7Interactable`))
            (for _array_element (`self.ConnectedWires`)
              (message `/Game/BluePrints/RobertBlueprints/BPI_Interactables.ActivateColor` _array_element))))))))

(event `self.BoxCollision.OnComponentEndOverlap`
  (params (OverlappedComponent :type "PrimitiveComponent Object Reference") (OtherActor :type "Actor Object Reference") (OtherComp :type "PrimitiveComponent Object Reference") (OtherBodyIndex :type Integer))
  ;[1 1 1] Collision handling
  (`/Engine/EditorBlueprintResources/StandardMacros.IsValid` (`self.GetComponentByClass` OtherActor "/Script/GP3.T7InteractableTrigger")
    (:`Is Valid`
      (bind _result (`/Engine/EditorBlueprintResources/StandardMacros.DecrementInt` (`self.OverlapCount`))
        (:`  `
          (if (<= _result 0)
            (`T7InteractableComponent.TriggerDeactivate` (`self.T7Interactable`))
            (set `self.OverlapCount` 0)
            (for _array_element (`self.ConnectedWires`)
              (message `/Game/BluePrints/RobertBlueprints/BPI_Interactables.DeactivateColor` _array_element))))))))

(fn `UserConstructionScript`)