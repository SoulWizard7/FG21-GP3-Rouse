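; BP_PuzzleBreakableFloor is an interactable puzzle floor that disappears when activated.
; It responds to T7InteractableResponse activation by hiding the Floor component and disabling its collision.
; Deactivation restores visibility and query-and-physics collision only when the DoDeactivate flag is set, so the break can be permanent or reversible.
; Both responses print debug strings.
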(event `self.T7InteractableResponse.OnActivate`
  (bind _floor (`self.Floor`))
  (`KismetSystemLibrary.PrintString` "Activate!")
  (`SceneComponent.SetHiddenInGame` _floor true false)
  (`PrimitiveComponent.SetCollisionEnabled` _floor "NoCollision"))

(event `self.T7InteractableResponse.OnDeactivate`
  (bind _floor (`self.Floor`))
  (if (`self.DoDeactivate`)
    (`KismetSystemLibrary.PrintString` "Deactivate!")
    (`SceneComponent.SetHiddenInGame` _floor false false)
    (`PrimitiveComponent.SetCollisionEnabled` _floor "QueryAndPhysics")))

(fn `UserConstructionScript`)