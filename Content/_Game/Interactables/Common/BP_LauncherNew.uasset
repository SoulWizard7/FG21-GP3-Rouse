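; BP_LauncherNew is a launcher that repeatedly fires a single physics dice (BP_Interactable_Small).
; On BeginPlay it spawns the dice at DiceSpawnPoint and applies an impulse along ImpulseDirection, scaled by ImpulseForce.
; When that dice overlaps DiceDestroyCollider, it is recycled rather than destroyed: its ammo is retracted, it teleports back, its velocity is zeroed and it relaunches.
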(event `self.ReceiveBeginPlay`
  (bind _impulseforce (`self.ImpulseForce`))
  (set `self.ImpulseVector` (* (`SceneComponent.GetForwardVector` (`self.ImpulseDirection`)) (`KismetMathLibrary.MakeVector` _impulseforce _impulseforce _impulseforce)))
  (bind _returnvalue (`|SpawnActorFromClass` "/Game/_Game/Interactables/Gun/BP_Interactable_Small.BP_Interactable_Small_C" (`SceneComponent.K2_GetComponentToWorld` (`self.DiceSpawnPoint`)) "Undefined" "OverrideRootScale" null null))
  (bind _output_get (set `self.CurrentDice` _returnvalue))
  (`PrimitiveComponent.AddImpulse` (`/Game/_Game/Interactables/Gun/BP_GunInteractableBase.Cube` _output_get) (`self.ImpulseVector`) "None" false))

(event `self.DiceDestroyCollider.OnComponentBeginOverlap`
  (params (OverlappedComponent :type "PrimitiveComponent Object Reference") (OtherActor :type "Actor Object Reference") (OtherComp :type "PrimitiveComponent Object Reference") (OtherBodyIndex :type Integer) (bFromSweep :type Boolean) (SweepResult :type "HitResult Structure (by ref)"))
  (bind _currentdice (`self.CurrentDice`))
  (if (== OtherActor _currentdice)
    (`/Game/_Game/Interactables/Gun/BP_GunInteractableBase.RetractAmmo` _currentdice)
    (`SceneComponent.K2_SetWorldTransform` (`Actor.RootComponent` (`self.CurrentDice`)) (`SceneComponent.K2_GetComponentToWorld` (`self.DiceSpawnPoint`)) false true)
    (`PrimitiveComponent.SetAllPhysicsLinearVelocity` (`/Game/_Game/Interactables/Gun/BP_GunInteractableBase.Cube` (`self.CurrentDice`)) (0.0 0.0 0.0) false)
    (`PrimitiveComponent.AddImpulse` (`/Game/_Game/Interactables/Gun/BP_GunInteractableBase.Cube` (`self.CurrentDice`)) (`self.ImpulseVector`) "None" false)
    (`KismetSystemLibrary.PrintString` "cube respawn" true true (struct :`G` 0.66 :`B` 1.0 :`A` 1.0) 1.0)))

(fn `UserConstructionScript`)